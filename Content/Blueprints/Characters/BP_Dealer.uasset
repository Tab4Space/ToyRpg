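; BP_Dealer is a prototype dealer character with four skill events, A to D, which are placeholders that only print messages.
; Tick, throttled by a short Delay, refreshes combat state with random stand-ins for own, teammate and monster HP and most distances.
; Only the distance to the first teammate is measured, using BPSupporter's location.
; Unconnected nodes sketch turning the actor and controller yaw toward BPSupporter.
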(event `self.Activate_Skill_A`
  ;[1 1 1] 코멘트
  (`KismetSystemLibrary.PrintString` "ACtivate Skill A"))

(event `self.ReceiveTick`
  (params (DeltaSeconds :type "Float (single-precision)"))
  (`KismetSystemLibrary.Delay` 0.1)
  (`|ExecutionSequence`
    (:`then_0`
      (set `self.CharacterHP` (`KismetMathLibrary.RandomFloat`)))
    (:`then_1`
      (set `self.MyTeamHP1` (`KismetMathLibrary.RandomFloat`)))
    (:`then_2`
      (set `self.MyTeamHP2` (`KismetMathLibrary.RandomFloat`)))
    (:`then_3`
      (set `self.MonsterHP` (`KismetMathLibrary.RandomFloat`)))
    (:`then_4`
      (set `self.DistanceMeToMonster` (`KismetMathLibrary.RandomFloat`)))
    (:`then_5`
      (set `self.DistanceMeToTeam1` (`KismetMathLibrary.Vector_Distance` (`self.K2_GetActorLocation`) (`self.K2_GetActorLocation` (`self.BP_Supporter`)))))
    (:`then_6`
      (set `self.DistanceMeToTeam2` (`KismetMathLibrary.RandomFloat`)))))

(event `self.Activate_Skill_B`
  ;[1 1 1] 코멘트
  (`KismetSystemLibrary.PrintString` "ACtivate Skill B"))

(event `self.Activate_Skill_C`
  ;[1 1 1] 코멘트
  (`KismetSystemLibrary.PrintString` "ACtivate Skill C"))

(event `self.Activate_Skill_D`
  ;[1 1 1] 코멘트
  (`KismetSystemLibrary.PrintString` "ACtivate Skill D"))

(fn `UserConstructionScript`)